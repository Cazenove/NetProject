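; PC_Lobby is the lobby player controller for a networked game's session room.
; On BeginPlay it reads PlayerInfo from NetGameInstance, shows the W_Lobby widget with cursor and Game-and-UI input, then registers the player with GM_Lobby.
; It forwards player-info changes and refresh requests to GM_Lobby and exposes UpdateInfo to refresh the widget's player and map display.
; LeaveRoom destroys the session and opens WelcomMap on success.
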(event Custom|Init
  ;[1 1 1] 初始化
  (bind _asnet_game_instance (Utilities|Casting|CastToNetGameInstance (Game|GetGameInstance)))
  (Variables|Default|SetPlayerInfo (Variables|/Game/Blueprints/NetGameInstance.NetGameInstance_C|GetPlayerInfo _asnet_game_instance))
  (CallFunction|ShowReadyUI))

(event Custom|ShowReadyUI
  (bind _self self)
  ;[1 1 1] 显示UI
  (bind _returnvalue (UserInterface|CreateWidget "/Game/Blueprints/UI/W_Lobby.W_Lobby_C" _self))
  (bind _output_get (Variables|Default|SetLobbyUI _returnvalue))
  (UserInterface|Viewport|AddtoViewport _output_get 0)
  (Variables|/Script/Engine.PlayerController|SetbShowMouseCursor _self true)
  (Input|SetInputModeGameandUI _self (Variables|Default|GetLobbyUI) "DoNotLock" true)
  (Default|Init (Variables|Default|GetLobbyUI))
  (CallFunction|AddPlayerInfo (Variables|Default|GetPlayerInfo))
  (CallFunction|UpdateAllPlayer))

(event Custom|UpdateInfo
  (params (PlayerInfo :type Array%20of%20Str%20Player%20Info%20Structures) (MapName :type Text))
  (bind _lobbyui (Variables|Default|GetLobbyUI))
  ;[1 1 1] 更新自身大厅控件信息
  (Default|UpdateInfo _lobbyui PlayerInfo)
  (Default|UpdateMapName _lobbyui MapName))

(event Custom|UpdateAllPlayer
  ;[1 1 1] 更新所有玩家
  (bind _asgm_lobby (Utilities|Casting|CastToGM_Lobby (Game|GetGameMode)))
  (Default|UpdateAllPlayer _asgm_lobby))

(event Custom|AddPlayerInfo
  (params (PlayerInfo :type Str%20Player%20Info%20Structure))
  ;[1 1 1] 添加玩家信息
  (bind _asgm_lobby (Utilities|Casting|CastToGM_Lobby (Game|GetGameMode)))
  (Default|AddPlayerInfo _asgm_lobby PlayerInfo))

(event Custom|UpdatePlayerInfo
  (params (PlayerInfo :type Str%20Player%20Info%20Structure))
  ;[1 1 1] 更新玩家信息
  (bind _asgm_lobby (Utilities|Casting|CastToGM_Lobby (Game|GetGameMode)))
  (Default|UpdatePlayerInfo _asgm_lobby PlayerInfo))

(event Custom|LeaveRoom
  (|DestroySession self
    (:OnSuccess
      (Development|PrintString "离开成功")
      (Game|OpenLevel(byName) "WelcomMap"))
    (:OnFailure
      (Development|PrintString "离开失败"))))

(event EventBeginPlay
  ;[1 1 1] 开始
  (CallFunction|Init))

(event EventTick
  (params (DeltaSeconds :type Float%20%28single-precision%29)))

(fn ConstructionScript)