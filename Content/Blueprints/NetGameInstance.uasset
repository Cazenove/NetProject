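; NetGameInstance, by its name a Game Instance, opens the create-room and room-list screens for what appears to be a multiplayer lobby.
; OpenCreateRoomUI and OpenRoomList each create their widget for player controller 0 on first use, cache it and add it to the viewport.
; Later calls make the cached widget visible again; no session or networking logic appears here.
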(event Custom|OpenCreateRoomUI
  (Utilities|IsValid (Variables|Default|GetCreateRoomUI)
    (:Is%20Valid
      (Widget|SetVisibility (Variables|Default|GetCreateRoomUI) "Visible"))
    (:Is%20Not%20Valid
      (bind _returnvalue (UserInterface|CreateWidget "/Game/Blueprints/UI/W_CreateRoom.W_CreateRoom_C" (Game|GetPlayerController 0)))
      (bind _output_get (Variables|Default|SetCreateRoomUI _returnvalue))
      (UserInterface|Viewport|AddtoViewport _output_get 0))))

(event Custom|OpenRoomList
  (Utilities|IsValid (Variables|Default|GetRoomListUI)
    (:Is%20Valid
      (Widget|SetVisibility (Variables|Default|GetRoomListUI) "Visible"))
    (:Is%20Not%20Valid
      (bind _returnvalue (UserInterface|CreateWidget "/Game/Blueprints/UI/W_RoomList.W_RoomList_C" (Game|GetPlayerController 0)))
      (bind _output_get (Variables|Default|SetRoomListUI _returnvalue))
      (UserInterface|Viewport|AddtoViewport _output_get 0))))