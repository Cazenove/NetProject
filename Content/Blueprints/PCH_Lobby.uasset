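; PCH_Lobby is a lobby player pawn that tests Gameplay Ability System abilities, shooting and damage through input.
; Three ability inputs activate the first three MyAbilities classes on its AbilitySystem component, with remote activation allowed.
; Fire calls custom event CE1, which spawns BP_Bullet at the actor's transform with itself as owner.
; Debug prints report ability presses, damage received and, on Q, an attribute read labelled health on failure.
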(event Custom|CE1
  (bind _returnvalue (Transformation|GetActorTransform))
  (Game|SpawnActorfromClass "/Game/Blueprints/BP_Bullet.BP_Bullet_C" (Math|Transform|MakeTransform (.location _returnvalue) (.rotation _returnvalue) (.scale _returnvalue)) "Undefined" self 0))

(event EventBeginPlay)

(event Collision|EventActorBeginOverlap
  (params (OtherActor :type Actor%20Object%20Reference)))

(event EventTick
  (params (DeltaSeconds :type Float%20%28single-precision%29)))

(event Game|Damage|EventAnyDamage
  (params (Damage :type Float%20%28single-precision%29) (DamageType :type Damage%20Type%20Object%20Reference) (InstigatedBy :type Controller%20Object%20Reference) (DamageCauser :type Actor%20Object%20Reference))
  (Development|PrintString (Utilities|String|ToString(Float) Damage)))

(event Input|ActionEvents|InputActionUseAbility1
  (params (Key :type Key%20Structure :default "None"))
  (:Pressed
    (Development|PrintString "UseAbility1")
    (Abilities|TryActivateAbilitybyClass (Variables|Default|GetAbilitySystem) (Utilities|Array|Get(acopy) (Variables|Default|GetMyAbilities)) true)))

(event Input|ActionEvents|InputActionUseAbility2
  (params (Key :type Key%20Structure :default "None"))
  (:Pressed
    (Development|PrintString "UseAbility2")
    (Abilities|TryActivateAbilitybyClass (Variables|Default|GetAbilitySystem) (Utilities|Array|Get(acopy) (Variables|Default|GetMyAbilities) 1) true)))

(event Input|ActionEvents|InputActionUseAbility3
  (params (Key :type Key%20Structure :default "None"))
  (:Pressed
    (Development|PrintString "UseAbility3")
    (Abilities|TryActivateAbilitybyClass (Variables|Default|GetAbilitySystem) (Utilities|Array|Get(acopy) (Variables|Default|GetMyAbilities) 2) true)))

(event Input|ActionEvents|InputActionFire
  (params (Key :type Key%20Structure :default "None"))
  (:Pressed
    (CallFunction|CE1)))

(event Input|KeyboardEvents|Q
  (params (Key :type Key%20Structure :default "None"))
  (bind _abilitysystem (Variables|Default|GetAbilitySystem))
  (bind (_bsuccessfullyfoundattribute _returnvalue) (Ability|Attribute|GetFloatAttributefromAbilitySystemComponent _abilitysystem "(AttributeName=\"Health\",Attribute=/Script/NetProject.AttributeSet1:Health,AttributeOwner=None)"))
  (:Pressed
    (if _bsuccessfullyfoundattribute
      (Development|PrintString (Utilities|String|ToString(Float) _returnvalue))
      (else
        (Development|PrintString "读取health失败")))))

(fn ConstructionScript)