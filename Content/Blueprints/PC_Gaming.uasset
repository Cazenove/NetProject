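; PC_Gaming is a player controller that sets up the gameplay UI and tracks a Health value.
; On BeginPlay, a custom Init event creates the UI_Gaming widget with itself as owning player and adds it to the viewport.
; AnyDamage subtracts incoming damage from Health and prints the result, with no clamping, death handling or direct widget update.
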(event Custom|AnyDamage
  (params (Damage :type Float%20%28single-precision%29))
  (bind _output_get (Variables|Default|SetHealth (- (Variables|Default|GetHealth) Damage)))
  (Development|PrintString (Utilities|String|ToString(Float) _output_get)))

(event Custom|Init
  (bind _returnvalue (UserInterface|CreateWidget "/Game/Blueprints/UI/UI_Gaming.UI_Gaming_C" self))
  (UserInterface|Viewport|AddtoViewport _returnvalue 0))

(event EventBeginPlay
  (CallFunction|Init))

(fn ConstructionScript)