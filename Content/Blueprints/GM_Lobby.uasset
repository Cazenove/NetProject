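; Lobby game mode that records players as they log in and gives each a lobby pawn.
; On BeginPlay, the server caches the checkpoint map name from NetGameInstance.
; PostLogin adds each controller to PlayerList and calls SpawnPlayer, which spawns a pawn at the first PlayerStart found and possesses it.
; If the controller already has a pawn, DestroyActor runs untargeted, on the game mode itself rather than that pawn.
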(event Custom|SpawnPlayer
  (params (Controller :type Player%20Controller%20Object%20Reference))
  ;[1 1 1] 生成玩家
  (Utilities|IsValid (Pawn|GetControlledPawn Controller)
    (:Is%20Valid
      (Actor|DestroyActor))
    (:Is%20Not%20Valid
      _))
  (bind _outactors (Actor|GetAllActorsOfClass "/Script/Engine.PlayerStart"))
  (bind _returnvalue (Game|SpawnActorfromClass "/Game/Blueprints/PCH_Lobby.PCH_Lobby_C" (Transformation|GetActorTransform (Utilities|Array|Get(acopy) _outactors)) "AdjustIfPossibleButAlwaysSpawn" 0 0))
  (Pawn|Possess Controller _returnvalue))

(event EventBeginPlay
  ;[1 1 1] 保存关卡信息
  (Networking|SwitchHasAuthority
    (:Authority
      (bind _asnet_game_instance (Utilities|Casting|CastToNetGameInstance (Game|GetGameInstance)))
      (Variables|Default|SetMapName (Variables|/Game/Blueprints/NetGameInstance.NetGameInstance_C|GetCheckPointName _asnet_game_instance)))))

(event EventTick
  (params (DeltaSeconds :type Float%20%28single-precision%29)))

(event EventPostLogin
  (params (NewPlayer :type Player%20Controller%20Object%20Reference))
  ;[1 1 1] 玩家登陆
  (Networking|SwitchHasAuthority
    (:Authority
      (Utilities|Array|Add (Variables|Default|GetPlayerList) NewPlayer)
      (CallFunction|SpawnPlayer NewPlayer))))

(fn ConstructionScript)