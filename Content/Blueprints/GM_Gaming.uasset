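; GM_Gaming is a game mode that spawns a character for each joining player and can move the session to another map.
; On PostLogin it records the controller in PlayerList, then spawns and possesses a ThirdPersonCharacter at the PlayerStart indexed by an incrementing PlayerNum, with no bounds check.
; OpenNewLevel runs a ServerTravel console command to NewWorld through the first player controller.
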(event Custom|OpenNewLevel
  (Development|ExecuteConsoleCommand "ServerTravel NewWorld" (Game|GetPlayerController 0)))

(event EventBeginPlay)

(event EventTick
  (params (DeltaSeconds :type Float%20%28single-precision%29)))

(event EventPostLogin
  (params (NewPlayer :type Player%20Controller%20Object%20Reference))
  (Utilities|Array|Add (Variables|Default|GetPlayerList) NewPlayer)
  (bind _outactors (Actor|GetAllActorsOfClass "/Script/Engine.PlayerStart"))
  (bind _returnvalue (Game|SpawnActorfromClass "/Game/ThirdPersonCPP/Blueprints/ThirdPersonCharacter.ThirdPersonCharacter_C" (Math|Transform|MakeTransform (.location (Transformation|GetActorTransform (Utilities|Array|Get(acopy) _outactors (Variables|Default|GetPlayerNum)))) (.rotation (Transformation|GetActorTransform (Utilities|Array|Get(acopy) _outactors (Variables|Default|GetPlayerNum)))) "1,1,1") "Undefined" 0 0))
  (Pawn|Possess NewPlayer _returnvalue)
  (Math|Integer|IncrementInt (Variables|Default|GetPlayerNum)))

(fn ConstructionScript)