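; BP_Bullet is a projectile actor that damages third-person characters it hits and explodes on impact.
; On BeginPlay it sets the ProjectileMovement velocity along its forward vector, scaled by InitVelocity.
; On a hit with anything other than its owner, it applies fixed damage if the target is a ThirdPersonCharacter, then destroys itself and spawns an explosion emitter at the hit location.
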(event EventBeginPlay
  (Variables|/Script/Engine.MovementComponent|SetVelocity (Variables|Default|GetProjectileMovement) (* (Transformation|GetActorForwardVector) (Variables|Default|GetInitVelocity))))

(event Collision|EventHit
  (params (MyComp :type Primitive%20Component%20Object%20Reference) (Other :type Actor%20Object%20Reference) (OtherComp :type Primitive%20Component%20Object%20Reference) (bSelfMoved :type Boolean) (HitLocation :type Vector :default "0, 0, 0") (HitNormal :type Vector :default "0, 0, 0") (NormalImpulse :type Vector :default "0, 0, 0") (Hit :type Hit%20Result%20Structure%20%28by%20ref%29))
  (if (!= Other (Components|GetOwner))
    (bind _asthird_person_character (Utilities|Casting|CastToThirdPersonCharacter Other)
      (:then
        (Game|Damage|ApplyDamage _asthird_person_character 5e+01 0 0))
      (:CastFailed
        _))
    (Actor|DestroyActor)
    (Effects|SpawnEmitteratLocation "/Game/StarterContent/Particles/P_Explosion.P_Explosion" HitLocation)))

(fn ConstructionScript)